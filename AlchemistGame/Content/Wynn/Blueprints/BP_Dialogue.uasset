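; BP_Dialogue is an interactable Blueprint that steps through lines of dialogue on a text render component.
; Each Interact event increments TalkIndex, then shows that entry of the Dialogue array as the render text.
; The index check uses less-than-or-equal against the array length, so it also lets an index one past the last entry through.
; Nothing in the graph resets the index or clears the text.
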(event `/Game/Wynn/Blueprints/BPI_Interact.Interact`
  (`/Engine/EditorBlueprintResources/StandardMacros.IncrementInt` (`self.talkIndex`)
    (:`  `
      (if (<= (`self.talkIndex`) (`KismetArrayLibrary.Array_Length` (`self.dialogue`)))
        (`TextRenderComponent.K2_SetText` (`self.TextRender`) (`KismetTextLibrary.Conv_StringToText` (`|GetArrayItem` (`self.dialogue`) (`self.talkIndex`))))))))

(fn `UserConstructionScript`)