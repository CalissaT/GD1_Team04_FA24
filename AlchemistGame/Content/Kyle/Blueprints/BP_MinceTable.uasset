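; BP_MinceTable is a table actor that detects mincable objects and players near it, with the mincing logic still unimplemented.
; The ObjectHold overlap stores any actor confirmed by IsMincableMessage in ObjectHolding and calls HoldObj, which so far only checks validity.
; The AtTableTrigger overlap uses message calls to tell players when they enter or leave the table.
; MinceObj is an empty stub.
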(event `self.ObjectHold.OnComponentBeginOverlap`
  (params (OverlappedComponent :type "PrimitiveComponent Object Reference") (OtherActor :type "Actor Object Reference") (OtherComp :type "PrimitiveComponent Object Reference") (OtherBodyIndex :type Integer) (bFromSweep :type Boolean) (SweepResult :type "HitResult Structure (by ref)"))
  (bind _canmince (message `/Game/Kyle/Blueprints/ActionableObj.IsMincable` OtherActor))
  (if _canmince
    (set `self.objectHolding` OtherActor)
    (`self.HoldObj`)))

(event `self.AtTableTrigger.OnComponentBeginOverlap`
  (params (OverlappedComponent :type "PrimitiveComponent Object Reference") (OtherActor :type "Actor Object Reference") (OtherComp :type "PrimitiveComponent Object Reference") (OtherBodyIndex :type Integer) (bFromSweep :type Boolean) (SweepResult :type "HitResult Structure (by ref)"))
  (bind _isplayer (message `/Game/Kyle/Blueprints/BPI_Player.isPlayer` OtherActor))
  (if _isplayer
    (message `/Game/Kyle/Blueprints/BPI_Player.setAtTable` OtherActor)))

(event `self.AtTableTrigger.OnComponentEndOverlap`
  (params (OverlappedComponent :type "PrimitiveComponent Object Reference") (OtherActor :type "Actor Object Reference") (OtherComp :type "PrimitiveComponent Object Reference") (OtherBodyIndex :type Integer))
  (bind _isplayer (message `/Game/Kyle/Blueprints/BPI_Player.isPlayer` OtherActor))
  (if _isplayer
    (message `/Game/Kyle/Blueprints/BPI_Player.setNotAtTable` OtherActor)))

(fn `HoldObj`
  ;[1 1 1] make it so you cant move it off the position lol
  (if (`KismetSystemLibrary.IsValid` (`self.objectHolding`))
    _))

(fn `MinceObj`)

(fn `UserConstructionScript`)